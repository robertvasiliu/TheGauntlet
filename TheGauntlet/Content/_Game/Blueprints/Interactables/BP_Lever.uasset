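; BP_Lever is an interactable lever that toggles an on/off state and reports each use to GauntletGameMode.
; Box overlap sets or clears itself as the Gauntlet character's CurrentLever.
; Interact calls UseLever, which flips IsOn, picks one of two fixed mesh rotations from the actor's roll rather than IsOn, then calls RegisterLeverState.
; IsLeverOn exposes the current state.
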(event OnComponentBeginOverlap(Box)
  (params (OverlappedComponent :type Primitive%20Component%20Object%20Reference) (OtherActor :type Actor%20Object%20Reference) (OtherComp :type Primitive%20Component%20Object%20Reference) (OtherBodyIndex :type Integer) (bFromSweep :type Boolean) (SweepResult :type Hit%20Result%20Structure%20%28by%20ref%29))
  (bind _asbp_the_gauntlet_character (Utilities|Casting|CastToBP_TheGauntletCharacter OtherActor))
  (Variables|/Game/_Game/Core/BP_TheGauntletCharacter.BP_TheGauntletCharacter_C|SetCurrentLever _asbp_the_gauntlet_character self))

(event OnComponentEndOverlap(Box)
  (params (OverlappedComponent :type Primitive%20Component%20Object%20Reference) (OtherActor :type Actor%20Object%20Reference) (OtherComp :type Primitive%20Component%20Object%20Reference) (OtherBodyIndex :type Integer))
  (bind _asbp_the_gauntlet_character (Utilities|Casting|CastToBP_TheGauntletCharacter OtherActor))
  (Variables|/Game/_Game/Core/BP_TheGauntletCharacter.BP_TheGauntletCharacter_C|SetCurrentLever _asbp_the_gauntlet_character 0))

(event Custom|UseLever
  (Variables|Default|SetbIsOn (not (Variables|Default|GetbIsOn)))
  (if (Math|Float|NearlyEqual(Float) (.Roll (Math|Rotator|BreakRotator (Transformation|GetActorRotation))) 0.0 1e-06)
    (Transformation|SetRelativeRotation (Variables|Default|GetStaticMesh) "0.000000,180.000000,120.000000" false false)
    (bind _asgauntlet_game_mode (Utilities|Casting|CastToGauntletGameMode (Game|GetGameMode)))
    (Class|GauntletGameMode|RegisterLeverState _asgauntlet_game_mode)
    (else
      (Transformation|SetRelativeRotation (Variables|Default|GetStaticMesh) "0.000000,180.000000,30.000000" false false)
      (bind _asgauntlet_game_mode_2 (Utilities|Casting|CastToGauntletGameMode (Game|GetGameMode)))
      (Class|GauntletGameMode|RegisterLeverState _asgauntlet_game_mode_2))))

(event EventInteract
  (params (InstigatorCharacter :type BP%20the%20Gauntlet%20Character%20Object%20Reference))
  (CallFunction|UseLever))

(fn ConstructionScript)

(fn IsLeveron
  (return (Variables|Default|GetbIsOn)))