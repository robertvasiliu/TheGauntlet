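; BP_Destructible is an interactable object that loses health with each interaction and is destroyed when it runs out.
; A box trigger tracks whether the BP_TheGauntletCharacter is in range through PlayerInRange, which this graph sets but never checks.
; The Interact event calls TakeInteractHit, which subtracts a fixed amount of Health and destroys the actor at zero or below.
; Debug strings print on overlap changes and on destruction.
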(event OnComponentBeginOverlap(Box)
  (params (OverlappedComponent :type Primitive%20Component%20Object%20Reference) (OtherActor :type Actor%20Object%20Reference) (OtherComp :type Primitive%20Component%20Object%20Reference) (OtherBodyIndex :type Integer) (bFromSweep :type Boolean) (SweepResult :type Hit%20Result%20Structure%20%28by%20ref%29))
  (Utilities|Casting|CastToBP_TheGauntletCharacter OtherActor)
  (Variables|Default|SetbPlayerInRange true)
  (Development|PrintString "1"))

(event OnComponentEndOverlap(Box)
  (params (OverlappedComponent :type Primitive%20Component%20Object%20Reference) (OtherActor :type Actor%20Object%20Reference) (OtherComp :type Primitive%20Component%20Object%20Reference) (OtherBodyIndex :type Integer))
  (Utilities|Casting|CastToBP_TheGauntletCharacter OtherActor)
  (Variables|Default|SetbPlayerInRange false)
  (Development|PrintString "2"))

(event Custom|TakeInteractHit
  (bind _output_get (Variables|Default|SetHealth (- (Variables|Default|GetHealth) 1e+01)))
  (if (<= _output_get 0.0)
    (Actor|DestroyActor)
    (Development|PrintString "3")))

(event EventInteract
  (params (InstigatorCharacter :type BP%20the%20Gauntlet%20Character%20Object%20Reference))
  (CallFunction|TakeInteractHit))

(event Collision|EventActorBeginOverlap
  (params (OtherActor :type Actor%20Object%20Reference)))

(fn ConstructionScript)