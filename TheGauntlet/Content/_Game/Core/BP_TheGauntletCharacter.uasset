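; Player character Blueprint that handles movement, look, jump, interaction and pausing through Enhanced Input actions.
; Move, look and jump inputs forward to the DoMove, DoLook and jump functions.
; Interact runs a forward sphere trace on Visibility and sends InteractMessage to a hit actor implementing BPI_Interactable.
; Esc, only in Level_01, toggles game pause, creating or removing WBP_PauseMenu and switching cursor visibility and input mode.
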(event Input|EnhancedActionEvents|EnhancedInputActionIA_Move
  (params (ActionValue :type Vector%202D%20Structure) (ElapsedSeconds :type Float%20%28double-precision%29) (TriggeredSeconds :type Float%20%28double-precision%29) (InputAction :type Input%20Action%20Object%20Reference :default "/Game/Input/Actions/IA_Move.IA_Move"))
  (bind (_x _y) (Math|Vector2D|BreakVector2D ActionValue))
  (Class|TheGauntletCharacter|DoMove _x _y))

(event Input|EnhancedActionEvents|EnhancedInputActionIA_Esc
  (params (ActionValue :type Boolean) (ElapsedSeconds :type Float%20%28double-precision%29) (TriggeredSeconds :type Float%20%28double-precision%29) (InputAction :type Input%20Action%20Object%20Reference :default "/Game/_Game/Blueprints/IA_Esc.IA_Esc"))
  (bind _returnvalue (Game|GetPlayerController 0))
  (bind _returnvalue_2 (Game|GetPlayerController 0))
  (bind _returnvalue_3 (Game|GetCurrentLevelName true))
  (if (Utilities|Enum|Equal(Enum) _returnvalue_3 "Level_01")
    (if (Variables|Default|GetbIsPaused)
      (Game|SetGamePaused false)
      (Widget|RemovefromParent (Variables|Default|GetWBP_PauseMenu))
      (bind _output_get (Variables|/Script/Engine.PlayerController|SetbShowMouseCursor _returnvalue false))
      (Input|SetInputModeGameOnly _returnvalue _output_get)
      (else
        (Game|SetGamePaused true)
        (bind _returnvalue_4 (UserInterface|CreateWidget "/Game/_Game/UI/WBP_PauseMenu.WBP_PauseMenu_C"))
        (bind _output_get_2 (Variables|Default|SetWBP_PauseMenu _returnvalue_4))
        (UserInterface|Viewport|AddtoViewport _returnvalue_4 0)
        (bind _output_get_3 (Variables|/Script/Engine.PlayerController|SetbShowMouseCursor _returnvalue_2 true))
        (Input|SetInputModeUIOnly _returnvalue_2 0 "DoNotLock" _output_get_3)))))

(event Input|EnhancedActionEvents|EnhancedInputActionIA_Jump
  (params (ActionValue :type Boolean) (ElapsedSeconds :type Float%20%28double-precision%29) (TriggeredSeconds :type Float%20%28double-precision%29) (InputAction :type Input%20Action%20Object%20Reference :default "/Game/Input/Actions/IA_Jump.IA_Jump"))
  (:Started
    (Class|TheGauntletCharacter|DoJumpStart))
  (:Canceled
    (Class|TheGauntletCharacter|DoJumpEnd)))

(event Input|EnhancedActionEvents|EnhancedInputActionIA_MouseLook
  (params (ActionValue :type Vector%202D%20Structure) (ElapsedSeconds :type Float%20%28double-precision%29) (TriggeredSeconds :type Float%20%28double-precision%29) (InputAction :type Input%20Action%20Object%20Reference :default "/Game/Input/Actions/IA_MouseLook.IA_MouseLook"))
  (bind (_x _y) (Math|Vector2D|BreakVector2D ActionValue))
  (Class|TheGauntletCharacter|DoLook _x _y))

(event Input|EnhancedActionEvents|EnhancedInputActionIA_Interact
  (params (ActionValue :type Boolean) (ElapsedSeconds :type Float%20%28double-precision%29) (TriggeredSeconds :type Float%20%28double-precision%29) (InputAction :type Input%20Action%20Object%20Reference :default "/Game/Variant_SideScrolling/Input/Actions/IA_Interact.IA_Interact"))
  (bind _returnvalue (Transformation|GetActorLocation))
  (:Started
    (bind (_outhit _returnvalue_2) (Collision|SphereTraceByChannel _returnvalue (+ _returnvalue (* (Transformation|GetActorForwardVector) (Variables|Default|GetNewVar))) 7e+01 "TraceTypeQuery1" false 0 "None"))
    (if _returnvalue_2
      (if (Utilities|DoesObjectImplementInterface (.HitActor (Collision|BreakHitResult _outhit)) "/Game/_Game/Core/BPI_Interactable.BPI_Interactable_C")
        (Class|BPIInteractable|Interact(Message) (.HitActor (Collision|BreakHitResult _outhit)) self)))))

(fn ConstructionScript)